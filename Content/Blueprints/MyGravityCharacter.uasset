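; MyGravityCharacter is a character Blueprint that highlights itself when it can be possessed and equips an axe tool.
; Each Tick runs DrawOutline, which toggles an outline overlay material on the third-person mesh based on CanBePossessed.
; Only the possessable branch continues to a DoOnce, which spawns the axe, stores it as ToolRef and attaches it to the first-person mesh's tool socket with a rotation offset.
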(event `self.ReceiveTick`
  (params (DeltaSeconds :type "Float (single-precision)"))
  (`self.DrawOutline`
    (:`Output`
      (`/Engine/EditorBlueprintResources/StandardMacros.DoOnce` false
        (:`Completed`
          (bind _returnvalue (`|SpawnActorFromClass` "/Game/Blueprints/AxeClass.AxeClass_C" (`SceneComponent.GetSocketTransform` (`self.FPMesh`) "Tool_Socket" "RTS_World") "Undefined" "MultiplyWithRoot" null null))
          (bind _output_get (set `self.Tool_Ref` _returnvalue))
          (`self.K2_AttachToComponent` _output_get (`self.FPMesh`) "Tool_Socket" "KeepWorld" "KeepWorld" "KeepWorld" true)
          (`SceneComponent.K2_SetRelativeRotation` (`/Game/Blueprints/AxeClass.SkeletalMesh` (`self.Tool_Ref`)) (struct :`Pitch` 20.0 :`Yaw` 60.0 :`Roll` -10.0) false false))))))

(fn `UserConstructionScript`)